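; Player combat component for BP_ThirdPersonCharacter, handling target lock and sword attacks.
; Lock input sphere-traces from the camera for a Pawn, attaches a marker actor to it and turns the controller toward it every tick.
; Attack input plays a combo montage that stops at each notify unless another press was buffered.
; A looping timer between begin/end trace events sweeps between sword points, applying damage throttled by a resetting DoOnce.
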(event Custom|Begin%20Damage%20Trace
  ;[0.15 0.15 0.15 0.5] Sword Traces
  (bind _returnvalue (Utilities|Time|SetTimerbyEvent (delegate Custom|Damage%20Trace) 0.01 true)))

(event Custom|Damage%20Trace
  (bind _playerb (Variables|Default|GetPlayerB))
  ;[0.15 0.15 0.15 0.5] Sword Traces
  (bind _outhit (Collision|SphereTraceForObjects (Transformation|GetWorldLocation (Variables|/Game/ThirdPerson/Blueprints/BP_ThirdPersonCharacter.BP_ThirdPersonCharacter_C|GetStart%20Sword%20Trace%20Pos _playerb)) (Transformation|GetWorldLocation (Variables|/Game/ThirdPerson/Blueprints/BP_ThirdPersonCharacter.BP_ThirdPersonCharacter_C|GetEnd%20Sword%20Trace%20Pos _playerb)) 2e+01 (Utilities|Array|MakeArray "ObjectTypeQuery3") false 0 "ForOneFrame"))
  (if true
    (Utilities|FlowControl|DoOnce false :!label _label
      (:Completed
        (Game|Damage|ApplyDamage (.HitActor (Collision|BreakHitResult _outhit)) (Variables|Default|GetswordDamage) 0 0)
        (Utilities|FlowControl|Delay 0.1)
        (goto _label Reset)))))

(event Custom|End%20Damage%20Trace
  ;[0.15 0.15 0.15 0.5] Sword Traces
  (if true
    (Utilities|Time|ClearandInvalidateTimerbyHandle (stale Custom|Begin%20Damage%20Trace _returnvalue))))

(event Input|EnhancedActionEvents|EnhancedInputActionIA_Lock
  (params (ActionValue :type Boolean) (ElapsedSeconds :type Float%20%28double-precision%29) (TriggeredSeconds :type Float%20%28double-precision%29) (InputAction :type Input%20Action%20Object%20Reference :default "/Game/Input/Actions/IA_Lock.IA_Lock"))
  (bind _returnvalue (Game|GetPlayerCameraManager 0))
  (bind _playerb (Variables|Default|GetPlayerB))
  (bind _playerb_2 (Variables|Default|GetPlayerB))
  (bind _transformcomponent (Variables|/Script/Engine.PlayerCameraManager|GetTransformComponent _returnvalue))
  (bind _charactermovement (Variables|/Script/Engine.Character|GetCharacterMovement _playerb_2))
  (bind _charactermovement_2 (Variables|/Script/Engine.Character|GetCharacterMovement _playerb))
  (bind _returnvalue_2 (Transformation|GetWorldLocation _transformcomponent))
  ;[0.07292 0.07292 0.07292 0.5] Target Lock
  (:Started
    (Variables|Default|GetTargetLockActor
      (:then
        (Variables|Default|SetTargetLockActor 0)
        (Variables|/Script/Engine.CharacterMovementComponent|SetbOrientRotationToMovement _charactermovement_2 true)
        (Variables|/Script/Engine.CharacterMovementComponent|SetbUseControllerDesiredRotation _charactermovement_2 false)
        (Actor|DestroyActor (Variables|Default|GetTargetLockWidget)))
      (:else
        (bind (_outhit _returnvalue_3) (Collision|SphereTraceForObjects (Math|Vector|MakeVector (.x _returnvalue_2) (.y _returnvalue_2) (.z _returnvalue_2)) (+ (Math|Vector|MakeVector (.x _returnvalue_2) (.y _returnvalue_2) (+ (.z _returnvalue_2) 2e+01)) (* (Math|Vector|GetForwardVector (Transformation|GetWorldRotation _transformcomponent)) 1e+03)) 1.5e+02 (Utilities|Array|MakeArray "ObjectTypeQuery3") false 0 "ForDuration" true "(R=1.000000,G=0.000000,B=0.000000,A=1.000000)" "(R=0.000000,G=1.000000,B=0.000000,A=1.000000)" 2.0))
        (if _returnvalue_3
          (Variables|Default|SetTargetLockActor (.HitActor (Collision|BreakHitResult _outhit)))
          (Variables|/Script/Engine.CharacterMovementComponent|SetbOrientRotationToMovement _charactermovement false)
          (Variables|/Script/Engine.CharacterMovementComponent|SetbUseControllerDesiredRotation _charactermovement true)
          (bind _returnvalue_4 (Game|SpawnActorfromClass "/Game/Blueprints/BP_TargetLockWidget.BP_TargetLockWidget_C" (Math|Transform|MakeTransform (Math|Vector|MakeVector (.x (.location (Transformation|GetActorTransform (Variables|Default|GetTargetLockActor)))) (.y (.location (Transformation|GetActorTransform (Variables|Default|GetTargetLockActor)))) (+ (.z (.location (Transformation|GetActorTransform (Variables|Default|GetTargetLockActor)))) 2e+01)) (.rotation (Transformation|GetActorTransform (Variables|Default|GetTargetLockActor))) "1.000000,1.000000,1.000000") "AlwaysSpawn" "MultiplyWithRoot" 0 0))
          (bind _output_get (Variables|Default|SetTargetLockWidget _returnvalue_4))
          (Transformation|AttachActorToActor _output_get (Variables|Default|GetTargetLockActor) "None" "SnapToTarget" "SnapToTarget" "SnapToTarget" true))))))

(event Input|EnhancedActionEvents|EnhancedInputActionIA_Attack
  (params (ActionValue :type Boolean) (ElapsedSeconds :type Float%20%28double-precision%29) (TriggeredSeconds :type Float%20%28double-precision%29) (InputAction :type Input%20Action%20Object%20Reference :default "/Game/Input/Actions/IA_Attack.IA_Attack"))
  ;[0.07292 0.07292 0.07292 0.5] Sword Combo Animation
  (:Started
    (if (not (Variables|Default|GetIsAttacking))
      (Variables|Default|SetIsAttacking true)
      (Animation|Montage|PlayMontage (Variables|/Script/Engine.Character|GetMesh (Variables|Default|GetPlayerB)) "/Game/Characters/Souls/Combat/SwordAttackCombo_Montage.SwordAttackCombo_Montage"
        (:OnCompleted
          (Variables|Default|SetIsAttacking false :!label _label)
          (Variables|Default|SetCombo false))
        (:OnInterrupted
          (goto _label))
        (:OnNotifyBegin
          (if (and (Variables|Default|GetIsAttacking) (Variables|Default|GetCombo))
            (Variables|Default|SetCombo false)
            (else
              (Animation|Montage|MontageStop (Components|SkeletalMesh|GetAnimInstance (Variables|/Script/Engine.Character|GetMesh (Variables|Default|GetPlayerB))) 0.2 "/Game/Characters/Souls/Combat/SwordAttackCombo_Montage.SwordAttackCombo_Montage")))))
      (else
        (Variables|Default|SetCombo true)))))

(event EventBeginPlay
  ;[0.07292 0.07292 0.07292 0.5] Get Player Class
  (bind _asbp_third_person_character (Utilities|Casting|CastToBP_ThirdPersonCharacter (Components|GetOwner)))
  (Variables|Default|SetPlayerB _asbp_third_person_character))

(event EventTick
  (params (DeltaSeconds :type Float%20%28single-precision%29))
  (bind _playerb (Variables|Default|GetPlayerB))
  (bind _targetlockactor (Variables|Default|GetTargetLockActor))
  (bind _returnvalue (Transformation|GetActorLocation _targetlockactor))
  (bind _returnvalue_2 (Transformation|GetActorLocation _playerb))
  (bind _returnvalue_3 (Math|Rotator|FindLookatRotation _returnvalue_2 _returnvalue))
  ;[0.07292 0.07292 0.07292 0.5] Target Lock
  ;;[0.07292 0.07292 0.07292 0.5] Target Lock Update
  (Variables|Default|GetTargetLockActor
    (:then
      (Pawn|SetControlRotation (Pawn|GetController (Variables|Default|GetPlayerB)) (Math|Rotator|MakeRotator (.roll _returnvalue_3) (+ (.pitch _returnvalue_3) -2e+01) (.yaw _returnvalue_3))))
    (:else)))